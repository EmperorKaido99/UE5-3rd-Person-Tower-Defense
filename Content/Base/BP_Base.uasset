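; BP_Base is the base actor that loses health when enemies reach it.
; A BP_Enemy entering its box notifies the player character, spawns an explosion at the base and is destroyed.
; The base subtracts the ApplyDamage return value from its own health and destroys itself at zero.
; Tick pushes the health ratio to a WB_BaseHealthBar widget component, cached on BeginPlay.
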(event OnComponentBeginOverlap(Box)
  (params (OverlappedComponent :type Primitive%20Component%20Object%20Reference) (OtherActor :type Actor%20Object%20Reference) (OtherComp :type Primitive%20Component%20Object%20Reference) (OtherBodyIndex :type Integer) (bFromSweep :type Boolean) (SweepResult :type Hit%20Result%20Structure%20%28by%20ref%29))
  (bind _asbp_enemy (Utilities|Casting|CastToBP_Enemy OtherActor))
  (Class|BPIDecreaseEnemy|DecreaseEnemy(Message) (Game|GetPlayerCharacter 0))
  (bind _returnvalue (Game|Damage|ApplyDamage self 1.0 0 0))
  (Effects|SpawnEmitteratLocation "/Game/InfinityBladeEffects/Effects/FX_Monsters/FX_Monster_Gruntling/Bomber/P_BomberExplode.P_BomberExplode" (Variables|Default|GetBase%20Location) "0, 0, 0" "10.000000,10.000000,10.000000")
  (Actor|DestroyActor _asbp_enemy)
  (if (> (Variables|Default|GetBase%20Health) 0.0)
    (bind _output_get (Variables|Default|SetBase%20Health (- (Variables|Default|GetBase%20Health) _returnvalue)))
    (Development|PrintString (Utilities|String|ToString(Float) _output_get))
    (if (<= _output_get 0.0)
      (Actor|DestroyActor))))

(event EventBeginPlay
  (bind _aswb_base_health_bar (Utilities|Casting|CastToWB_BaseHealthBar (UserInterface|GetUserWidgetObject (Variables|Default|GetBaseHealthBar))))
  (Variables|Default|SetAs%20WB%20Base%20Health%20Bar _aswb_base_health_bar))

(event Collision|EventActorBeginOverlap
  (params (OtherActor :type Actor%20Object%20Reference)))

(event EventTick
  (params (DeltaSeconds :type Float%20%28single-precision%29))
  (Progress|SetPercent (Variables|/Game/HUD/WB_BaseHealthBar.WB_BaseHealthBar_C|GetHealthBar (Variables|Default|GetAs%20WB%20Base%20Health%20Bar)) (/ (Variables|Default|GetBase%20Health) (Variables|Default|GetMaxBasehealth))))

(fn ConstructionScript)