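; BP_Enemy is an enemy character with health, an explosion death and an overhead health bar.
; Each tick it updates the WB_HealthBar percent from its health and turns the bar to face the player camera.
; AnyDamage subtracts health and, at zero, calls Death, which calls DecreaseEnemyMessage on the player character, spawns the explosion and destroys the actor.
; An EnemyPath function exposes its Path variable.
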(event Custom|Death
  (Class|BPIDecreaseEnemy|DecreaseEnemy(Message) (Game|GetPlayerCharacter 0))
  (Effects|SpawnEmitteratLocation "/Game/InfinityBladeEffects/Effects/FX_Monsters/FX_Monster_Gruntling/Bomber/P_BomberExplode.P_BomberExplode" (Transformation|GetWorldLocation (Variables|Character|GetMesh)) "0, 0, 0" "2.000000,2.000000,2.000000")
  (Actor|DestroyActor))

(event EventBeginPlay
  (bind _aswb_health_bar (Utilities|Casting|CastToWB_HealthBar (UserInterface|GetUserWidgetObject (Variables|Default|GetHealthBar))))
  (Variables|Default|SetAs%20WB%20Health%20Bar _aswb_health_bar))

(event EventTick
  (params (DeltaSeconds :type Float%20%28single-precision%29))
  (bind _healthbar (Variables|Default|GetHealthBar))
  (Progress|SetPercent (Variables|/Game/HUD/WB_HealthBar.WB_HealthBar_C|GetHealthBar (Variables|Default|GetAs%20WB%20Health%20Bar)) (/ (Variables|Default|GetHealth) (Variables|Default|GetMaxhealth)))
  (Transformation|SetWorldRotation _healthbar (Math|Rotator|FindLookatRotation (Transformation|GetWorldLocation _healthbar) (Transformation|GetWorldLocation (Variables|/Script/Engine.PlayerCameraManager|GetTransformComponent (Game|GetPlayerCameraManager 0)))) false false))

(event Game|Damage|EventAnyDamage
  (params (Damage :type Float%20%28single-precision%29) (DamageType :type Damage%20Type%20Object%20Reference) (InstigatedBy :type Controller%20Object%20Reference) (DamageCauser :type Actor%20Object%20Reference))
  (if (> (Variables|Default|GetHealth) 0.0)
    (bind _output_get (Variables|Default|SetHealth (- (Variables|Default|GetHealth) Damage)))
    (if (<= _output_get 0.0)
      (CallFunction|Death))))

(fn ConstructionScript)

(fn EnemyPath
  (return (Variables|Default|GetPath)))